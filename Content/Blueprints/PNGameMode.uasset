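; Game mode Blueprint that respawns the player pawn and controls background music.
; On BeginPlay it binds to the player pawn's OnDestroyed and starts the BGM.
; When the pawn is destroyed, it spawns a new PNPlayerPawn at the player start, possesses it, rebinds the destroy event and restarts the music.
; PlayBGM swaps the track on a MusicSpeaker audio component at reduced volume.
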(event `self.ReceiveBeginPlay`
  (add `self.OnDestroyed` (`GameplayStatics.GetPlayerPawn` 0) (delegate `RespawnPlayer`))
  (`self.PlayBGM` "/Game/Audio/bgm02_Cue.bgm02_Cue"))

(event `RespawnPlayer` :!signature `self.OnDestroyed`
  (params (DestroyedActor :type "Actor Object Reference"))
  (bind _returnvalue (`|SpawnActorFromClass` "/Game/Blueprints/PNPlayerPawn.PNPlayerPawn_C" (`self.GetTransform` (`self.K2_FindPlayerStart` null)) "Undefined" "OverrideRootScale" null null))
  (`Controller.Possess` (`GameplayStatics.GetPlayerController` 0) _returnvalue)
  (add `self.OnDestroyed` _returnvalue (delegate `RespawnPlayer`))
  (`self.PlayBGM` "/Game/Audio/bgm02_Cue.bgm02_Cue"))

(fn `PlayBGM`
  (params (NewBGM :type "SoundCue Object Reference"))
  (`AudioComponent.Stop` (`self.MusicSpeaker`))
  (`AudioComponent.SetSound` (`self.MusicSpeaker`) NewBGM)
  (`AudioComponent.SetVolumeMultiplier` (`self.MusicSpeaker`) 0.5) ; 初期値だとうるさいのでまとめて設定する
  (`AudioComponent.Play` (`self.MusicSpeaker`) 0.0))

(fn `UserConstructionScript`)